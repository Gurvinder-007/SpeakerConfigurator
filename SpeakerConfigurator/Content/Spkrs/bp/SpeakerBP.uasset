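; Clickable speaker actor made of cabinet, woofers, horn tweeter, screen, frame, accent plate and feet meshes.
; Component clicks are grouped into accent, speaker, screen and cabinet events and forwarded to a referenced speaker logic Blueprint.
; InitializeSpeakerBP stores that reference and shows the screen and frame cover, or hides it and ignores its collision, based on CoverActive.
; Getter functions expose the meshes by group.
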(event OnClicked(HornTweeter)
  (params (TouchedComponent :type Primitive%20Component%20Object%20Reference) (ButtonPressed :type Key%20Structure :default "None"))
  ;[1 1 1] Speakers Clicked
  (Default|SpeakerClicked (Variables|Default|GetSpeaker_Logic_Reference)))

(event OnClicked(Woofers)
  (params (TouchedComponent :type Primitive%20Component%20Object%20Reference) (ButtonPressed :type Key%20Structure :default "None"))
  ;[1 1 1] Speakers Clicked
  (Default|SpeakerClicked (Variables|Default|GetSpeaker_Logic_Reference)))

(event OnClicked(AccentPlate)
  (params (TouchedComponent :type Primitive%20Component%20Object%20Reference) (ButtonPressed :type Key%20Structure :default "None"))
  ;[1 1 1] Accent Clicked
  (Default|AccentClicked (Variables|Default|GetSpeaker_Logic_Reference)))

(event OnClicked(Cabinette)
  (params (TouchedComponent :type Primitive%20Component%20Object%20Reference) (ButtonPressed :type Key%20Structure :default "None"))
  ;[1 1 1] Cabinet Clicked
  (Default|CabinetClicked (Variables|Default|GetSpeaker_Logic_Reference)))

(event OnClicked(Foot_BL)
  (params (TouchedComponent :type Primitive%20Component%20Object%20Reference) (ButtonPressed :type Key%20Structure :default "None"))
  ;[1 1 1] Accent Clicked
  (Default|AccentClicked (Variables|Default|GetSpeaker_Logic_Reference)))

(event OnClicked(Foot_BR)
  (params (TouchedComponent :type Primitive%20Component%20Object%20Reference) (ButtonPressed :type Key%20Structure :default "None"))
  ;[1 1 1] Accent Clicked
  (Default|AccentClicked (Variables|Default|GetSpeaker_Logic_Reference)))

(event OnClicked(Foot_FL)
  (params (TouchedComponent :type Primitive%20Component%20Object%20Reference) (ButtonPressed :type Key%20Structure :default "None"))
  ;[1 1 1] Accent Clicked
  (Default|AccentClicked (Variables|Default|GetSpeaker_Logic_Reference)))

(event OnClicked(Foot_FR)
  (params (TouchedComponent :type Primitive%20Component%20Object%20Reference) (ButtonPressed :type Key%20Structure :default "None"))
  ;[1 1 1] Accent Clicked
  (Default|AccentClicked (Variables|Default|GetSpeaker_Logic_Reference)))

(event OnClicked(Frame)
  (params (TouchedComponent :type Primitive%20Component%20Object%20Reference) (ButtonPressed :type Key%20Structure :default "None"))
  ;[1 1 1] Accent Clicked
  (Default|AccentClicked (Variables|Default|GetSpeaker_Logic_Reference)))

(event OnClicked(Screen)
  (params (TouchedComponent :type Primitive%20Component%20Object%20Reference) (ButtonPressed :type Key%20Structure :default "None"))
  ;[1 1 1] Screen Clicked
  (Default|ScreenClicked (Variables|Default|GetSpeaker_Logic_Reference)))

(event EventBeginPlay)

(event Collision|EventActorBeginOverlap
  (params (OtherActor :type Actor%20Object%20Reference)))

(event EventTick
  (params (DeltaSeconds :type Float%20%28single-precision%29)))

(fn ConstructionScript)

(fn GetCabineteComponent
  (return (Variables|Default|GetCabinette)))

(fn InitializeSpeakerBP
  (params (SpeakerLogicBP :type Speaker%20Logic%20BP%20Object%20Reference))
  (Utilities|FlowControl|Sequence
    (:then_0
      (Variables|Default|SetSpeaker_Logic_Reference SpeakerLogicBP))
    (:then_1
      ;[1 1 1] Check  Cover Active
      (if (Variables|Default|GetCover_Active)
        ;;[0.1684 1 0] Cover Is Active
        (Rendering|SetVisibility (Variables|Default|GetScreen) true false)
        (Rendering|SetVisibility (Variables|Default|GetFrame) true false)
        (else
          ;;[1 0 0] Cover Is Inactive
          (Rendering|SetVisibility (Variables|Default|GetScreen) false false)
          (Rendering|SetVisibility (Variables|Default|GetFrame) false false)
          (Collision|SetCollisionResponsetoAllChannels (Variables|Default|GetFrame) "ECR_Ignore")
          (Collision|SetCollisionResponsetoAllChannels (Variables|Default|GetScreen) "ECR_Ignore"))))))

(fn GetSpeakerComponents
  (return (Variables|Default|GetHornTweeter) (Variables|Default|GetWoofers)))

(fn GetAccentComponents
  (return (Utilities|Array|MakeArray (Variables|Default|GetFoot_BR) (Variables|Default|GetFoot_FL) (Variables|Default|GetFoot_FR) (Variables|Default|GetFoot_BL)) (Utilities|Array|MakeArray (Variables|Default|GetAccentPlate) (Variables|Default|GetFrame))))

(fn GetScreenComponent
  (return (Variables|Default|GetScreen)))