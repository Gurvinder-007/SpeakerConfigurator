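; Speaker configurator logic that cycles the finish of cabinet, driver, accent and screen parts on a list of speakers.
; Each Clicked function steps a wrapping index and picks a preset material set, or a color for the screen.
; Setter functions apply it to every speaker's components by swapping slot 0 materials, while the screen uses a "Color" vector parameter.
; InitializeSpeakerLogic receives the speaker list and a HUD reference.
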(event EventBeginPlay)

(event Collision|EventActorBeginOverlap
  (params (OtherActor :type Actor%20Object%20Reference)))

(event EventTick
  (params (DeltaSeconds :type Float%20%28single-precision%29)))

(fn ConstructionScript)

(fn CabinetClicked
  (bind _output_get (Variables|Default|SetCabinetIndex (Math|Integer|%(Integer) (+ (Variables|Default|GetCabinetIndex) 1) (Variables|Default|GetCabinetIndexMax))))
  (switch int _output_get
    (:0
      (CallFunction|SetCabinetMaterial "/Game/Spkrs/m/BlkGld_Cab.BlkGld_Cab"))
    (:1
      (CallFunction|SetCabinetMaterial "/Game/Spkrs/m/WalSlv_Cab.WalSlv_Cab"))
    (:2
      (CallFunction|SetCabinetMaterial "/Game/Spkrs/m/TkBlk_Cab.TkBlk_Cab"))
    (:3
      (CallFunction|SetCabinetMaterial "/Game/Spkrs/m/EbStl_Cab.EbStl_Cab"))
    (:4
      (CallFunction|SetCabinetMaterial "/Game/Spkrs/m/WhtCp_Cab.WhtCp_Cab"))))

(fn SetCabinetMaterial
  (params (Material :type Material%20Object%20Reference))
  (for _array_element (Variables|Default|GetSpeakerList)
    (bind _cabinetmesh (Default|GetCabineteComponent _array_element))
    (Rendering|Material|SetMaterial _cabinetmesh 0 Material)))

(fn InitializeSpeakerLogic
  (params (SpeakerList :type Array%20of%20Speaker%20BP%20Object%20References) (HUD :type HUD%20UI%20Object%20Reference))
  (Utilities|FlowControl|Sequence
    (:then_0
      (Variables|Default|SetSpeakerList SpeakerList))
    (:then_1
      (Variables|Default|SetHUD HUD))))

(fn SpeakerClicked
  (bind _output_get (Variables|Default|SetSpeakerIndex (Math|Integer|%(Integer) (+ (Variables|Default|GetSpeakerIndex) 1) (Variables|Default|GetSpeakerIndexMax))))
  (switch int _output_get
    (:0
      (CallFunction|SetSpeakerMaterials "/Game/Spkrs/m/BlkGld_Twt.BlkGld_Twt" "/Game/Spkrs/m/BlkGld_Wof.BlkGld_Wof"))
    (:1
      (CallFunction|SetSpeakerMaterials "/Game/Spkrs/m/WalSlv_Twt.WalSlv_Twt" "/Game/Spkrs/m/WalSlv_Wof.WalSlv_Wof"))
    (:2
      (CallFunction|SetSpeakerMaterials "/Game/Spkrs/m/TkBlk_Twt.TkBlk_Twt" "/Game/Spkrs/m/TkBlk_Wof.TkBlk_Wof"))
    (:3
      (CallFunction|SetSpeakerMaterials "/Game/Spkrs/m/WhtCP_Twt.WhtCP_Twt" "/Game/Spkrs/m/WhtCp_Wof.WhtCp_Wof"))))

(fn SetSpeakerMaterials
  (params (TweeterMaterial :type Material%20Object%20Reference) (WooferMaterial :type Material%20Object%20Reference))
  (for _array_element (Variables|Default|GetSpeakerList)
    (bind (_tweetermesh _woofermesh) (Default|GetSpeakerComponents _array_element))
    (Utilities|FlowControl|Sequence
      (:then_0
        (Rendering|Material|SetMaterial _tweetermesh 0 TweeterMaterial))
      (:then_1
        (Rendering|Material|SetMaterial _woofermesh 0 WooferMaterial)))))

(fn AccentClicked
  (bind _output_get (Variables|Default|SetAccentIndex (Math|Integer|%(Integer) (+ (Variables|Default|GetAccentIndex) 1) (Variables|Default|GetAccentIndexMax))))
  (switch int _output_get
    (:0
      ;[1 1 1] Comment
      (CallFunction|SetAccentMaterials "/Game/Spkrs/m/BlkGld_Ft.BlkGld_Ft" "/Game/Spkrs/m/BlkGld_Cab.BlkGld_Cab"))
    (:1
      (CallFunction|SetAccentMaterials "/Game/Spkrs/m/WalSlv_Ft.WalSlv_Ft" "/Game/Spkrs/m/WalSlv_Cab.WalSlv_Cab"))
    (:2
      (CallFunction|SetAccentMaterials "/Game/Spkrs/m/TkBlk_Ft.TkBlk_Ft" "/Game/Spkrs/m/TkBlk_Cab.TkBlk_Cab"))
    (:3
      (CallFunction|SetAccentMaterials "/Game/Spkrs/m/EbStl_Ft.EbStl_Ft" "/Game/Spkrs/m/EbStl_Cab.EbStl_Cab"))
    (:4
      (CallFunction|SetAccentMaterials "/Game/Spkrs/m/WhtCp_Ft.WhtCp_Ft" "/Game/Spkrs/m/WhtCp_Cab.WhtCp_Cab"))))

(fn SetAccentMaterials
  (params (FootMaterial :type Material%20Object%20Reference) (AccentMaterial :type Material%20Object%20Reference))
  (for _array_element (Variables|Default|GetSpeakerList)
    (bind (_footmeshes _accentmeshes) (Default|GetAccentComponents _array_element))
    (Utilities|FlowControl|Sequence
      (:then_0
        (for _array_element_2 _footmeshes
          (Rendering|Material|SetMaterial _array_element_2 0 FootMaterial)))
      (:then_1
        (for _array_element_3 _accentmeshes
          (Rendering|Material|SetMaterial _array_element_3 0 AccentMaterial))))))

(fn ScreenClicked
  (bind _output_get (Variables|Default|SetScreenIndex (Math|Integer|%(Integer) (+ (Variables|Default|GetScreenIndex) 1) (Variables|Default|GetScreenIndexMax))))
  (switch int _output_get
    (:0
      ;[0 0 0] Black
      (CallFunction|SetScreenColor "0, 0, 0"))
    (:1
      ;[0.1441 0.1155 0.0323] Gold
      (CallFunction|SetScreenColor "0.144100,0.115500,0.032300"))
    (:2
      ;[0.089 0.089 0.089] Dark Grey
      (CallFunction|SetScreenColor "0.089000,0.089000,0.089000"))
    (:3
      ;[1 1 1] White
      (CallFunction|SetScreenColor "1.000000,1.000000,1.000000"))
    (:4
      ;[0.0642 0.0237 0.0093] Dark Brown
      (CallFunction|SetScreenColor "0.064200,0.023700,0.009300"))))

(fn SetScreenColor
  (params (Color :type Vector))
  (for _array_element (Variables|Default|GetSpeakerList)
    (bind _screen_mesh (Default|GetScreenComponent _array_element))
    (Rendering|Material|SetVectorParameterValueonMaterials _screen_mesh "Color" Color)))